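; BP_camchanger is a trigger volume that switches the view to a fixed camera when the third person character enters it, as in fixed-angle camera games.
; On box overlap it moves the referenced camera actor to the configured position and rotation and stores it as the character's PreviousCamera.
; It then makes that camera the player controller's view target and aligns control rotation to it.
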(event `self.Box.OnComponentBeginOverlap`
  (params (OverlappedComponent :type "PrimitiveComponent Object Reference") (OtherActor :type "Actor Object Reference") (OtherComp :type "PrimitiveComponent Object Reference") (OtherBodyIndex :type Integer) (bFromSweep :type Boolean) (SweepResult :type "HitResult Structure (by ref)"))
  (bind _returnvalue (`GameplayStatics.GetPlayerController` 0))
  (bind _camera (`self.Camera`))
  (bind _asthird_person_character (cast `/Game/ThirdPersonBP/Blueprints/ThirdPersonCharacter` OtherActor))
  (bind _output_get (set `self.Camera` (`self.Camera`)))
  (`SceneComponent.K2_SetWorldLocationAndRotation` (`Actor.RootComponent` _output_get) (`self.Cam_pos`) (`self.Cam_Rotator`) false false)
  (set `/Game/ThirdPersonBP/Blueprints/ThirdPersonCharacter.Previous Camera` _camera _asthird_person_character)
  (`PlayerController.SetViewTargetWithBlend` _returnvalue _camera 0.0 "VTBlend_Linear" 0.0 false)
  (`Controller.SetControlRotation` _returnvalue (`self.K2_GetActorRotation` _camera)))

(fn `UserConstructionScript`)